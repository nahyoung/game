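; Castle floor actor whose floor mesh shows only while something overlaps its box trigger.
; The construction script uses Style to pick the floor and first-storey ceiling meshes from two arrays.
; At play start it hides the floor mesh, then box overlap begin and end toggle its visibility without filtering the actor or touching the ceiling.
; A leftover debug "Hello" prints on each overlap begin.
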(event OnComponentBeginOverlap(box)
  (params (OverlappedComponent :type Primitive%20Component%20Object%20Reference) (OtherActor :type Actor%20Object%20Reference) (OtherComp :type Primitive%20Component%20Object%20Reference) (OtherBodyIndex :type Integer) (bFromSweep :type Boolean) (SweepResult :type Hit%20Result%20Structure%20%28by%20ref%29))
  (Rendering|SetVisibility (Variables|Default|GetStaticMesh) true false)
  (Development|PrintString "Hello"))

(event OnComponentEndOverlap(box)
  (params (OverlappedComponent :type Primitive%20Component%20Object%20Reference) (OtherActor :type Actor%20Object%20Reference) (OtherComp :type Primitive%20Component%20Object%20Reference) (OtherBodyIndex :type Integer))
  (Rendering|SetVisibility (Variables|Default|GetStaticMesh) false false))

(event EventBeginPlay
  (Rendering|SetVisibility (Variables|Default|GetStaticMesh) false false))

(event Collision|EventActorBeginOverlap
  (params (OtherActor :type Actor%20Object%20Reference)))

(event EventTick
  (params (DeltaSeconds :type Float%20%28single-precision%29)))

(fn ConstructionScript
  (bind _style (Variables|Default|Getstyle))
  (Components|StaticMesh|SetStaticMesh (Variables|Default|GetStaticMesh) (Utilities|Array|Get(acopy) (Variables|Default|GetNew%20Floor) _style))
  (Components|StaticMesh|SetStaticMesh (Variables|Default|GetSm_ceil_1st) (Utilities|Array|Get(acopy) (Variables|Default|GetSm_ceil) _style)))